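; BP_GridBuilder is a grid generator actor meant to lay out typed map cells and size an interaction collision box.
; CalculateGridData holds logic that loads map data and builds an actor-centered, rotation-aligned cell array, tagging each Ground, Water or Hill.
; That logic and the SetCollisionBoxExtent sizing are disconnected from their function entries, so neither runs.
; Only SetGridGeneratorIndex, which stores the generator's index, is functional.
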(event `self.ReceiveBeginPlay`)

(fn `Calculate Grid Data`
  (params (GridCellSize :type "Float (double-precision)"))
  (returns (ReturnValue :type "Array of GridCellData Structure"))
  (locals (Local_GridCellSize :type "Float (double-precision)") (Local_GridCellData :type "Array of GridCellData Structure") (Local_StartingGridCellLocation :type "Vector Structure" :default (0.0 0.0 0.0)))
  ;[0 1 1 0.5] Calculates grid cell locations based on the grid cell size and number of grids along local x and y directions
)

(fn `SetCollisionBoxExtent`
  (params (GridCellSize :type "Float (double-precision)"))
  ;[0 1 1 0.5] Sets the size of the collision box based on the number of grid cells [Collision box can be used by players to interact with the grid generator]
)

(fn `SetGridGeneratorIndex`
  (params (Index :type Integer))
  (set `self.GeneratorIndex` Index)
  (return))

(fn `UserConstructionScript`
  (locals (Local_GridCellSize :type "Float (double-precision)" :default 0.0)))