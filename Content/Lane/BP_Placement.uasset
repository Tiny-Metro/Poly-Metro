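; BP_Placement is a placement preview actor for the lane system, displaying the mesh given by MeshType.
; It finds the LaneManager on BeginPlay and refreshes its mesh every Tick.
; Right-click cancels by destroying the actor, clearing the manager's placement validity and resetting its selected lane.
; Cursor-trace movement and the overlap-based material update exist but are disconnected, so neither runs.
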(event `self.ReceiveBeginPlay`
  (bind _returnvalue (`GameplayStatics.GetActorOfClass` "/Script/TinyMetro.LaneManager"))
  (set `self.LaneManagerRef` _returnvalue))

(event `self.ReceiveActorBeginOverlap`
  (params (OtherActor :type "Actor Object Reference")))

(event `self.ReceiveTick`
  (params (DeltaSeconds :type "Float (single-precision)"))
  (bind _lanemanagerref (`self.LaneManagerRef`))
  (`StaticMeshComponent.SetStaticMesh` (`self.StaticMesh`) (`self.MeshType`))
  (if (`PlayerController.WasInputKeyJustPressed` (`GameplayStatics.GetPlayerController` 0) "RightMouseButton")
    (`self.K2_DestroyActor`)
    (set `LaneManager.IsPlacementValid` false _lanemanagerref)
    (set `LaneManager.SelectedLaneNum` 0 _lanemanagerref)))

(fn `UpdateCollision`
  (if (== (`KismetArrayLibrary.Array_Length` (`self.GetOverlappingActors` null)) 0)
    (`PrimitiveComponent.SetMaterial` (`self.StaticMesh`) 0 null)
    (return)))

(fn `UserConstructionScript`)