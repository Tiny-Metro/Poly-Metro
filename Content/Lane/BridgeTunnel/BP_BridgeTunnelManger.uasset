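; Manager that creates and tracks bridge and tunnel connectors on the lane grid.
; Connects reuse an existing BP_BridgeTunnel by raising its count or spawn a new one, while disconnects lower that count.
; Connectors register and unregister in the BNT list, which FindBT searches by point set in either direction.
; On BeginPlay it finds the GridManager and connects the preset start points.
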(event `self.ReceiveBeginPlay`
  (bind _returnvalue (`GameplayStatics.GetActorOfClass` "/Script/TinyMetro.GridManager"))
  (set `self.GridManagerREF_0` _returnvalue)
  (for _array_element (`self.stpoit`)
    (`self.ConnectBT` (break `/Game/Lane/BridgeTunnel/ST_PointAr` _array_element))))

(event `CreateNewBT`
  (params (Point0 :type "Array of IntPoint Structure"))
  (bind (_x _y) (break `IntPoint` (`|GetArrayItem` Point0)))
  (bind (_returnvalue_index _returnvalue_worldcoordination _returnvalue_worldlocation) (break `GridCellData` (`GridManager.GetGridCellDataByPoint` (`self.GridManagerREF_0`) _x _y)))
  ;[1 1 1] BuildNewBT
  (bind _returnvalue (`|SpawnActorFromClass` "/Game/Lane/BridgeTunnel/BP_BridgeTunnel.BP_BridgeTunnel_C" (`KismetMathLibrary.MakeTransform` _returnvalue_worldlocation) "Undefined" "OverrideRootScale" null null))
  (`/Game/Lane/BridgeTunnel/BP_BridgeTunnel.SetBNT` _returnvalue (`self.GridManagerREF_0`) Point0 self "Bridge"))

(event `self.CreateNewBridge`
  (params (points :type "Array of IntPoint Structure (by ref)"))
  (`parent.CreateNewBridge` points)
  (bind _returnvalue (`|SpawnActorFromClass` "/Game/Lane/BridgeTunnel/BP_BridgeTunnel.BP_BridgeTunnel_C" (`KismetMathLibrary.MakeTransform` (0.0 0.0 -10.0)) "Undefined" "OverrideRootScale" null null))
  (`/Game/Lane/BridgeTunnel/BP_BridgeTunnel.SetBNT` _returnvalue (`self.GridManagerREF_0`) points self "Bridge"))

(event `getRegister`
  (params (ConnectorData :type "ConnectorData Structure"))
  (`KismetArrayLibrary.Array_AddUnique` (`self.BNT`) ConnectorData))

(event `getDeathCertificate`
  (params (ConnectorDat :type "ConnectorData Structure"))
  (`KismetArrayLibrary.Array_RemoveItem` (`self.BNT`) ConnectorDat))

(event `self.CreateNewTunnel`
  (params (points :type "Array of IntPoint Structure (by ref)"))
  (`parent.CreateNewTunnel` points)
  (bind _returnvalue (`|SpawnActorFromClass` "/Game/Lane/BridgeTunnel/BP_BridgeTunnel.BP_BridgeTunnel_C" (`KismetMathLibrary.MakeTransform` (0.0 0.0 -10.0)) "Undefined" "OverrideRootScale" null null))
  (`/Game/Lane/BridgeTunnel/BP_BridgeTunnel.SetBNT` _returnvalue (`self.GridManagerREF_0`) points self "Tunnel"))

(event `self.ConnectBT`
  (params (points :type "Array of IntPoint Structure (by ref)"))
  (`parent.ConnectBT` points)
  (bind (_doesexist _thebnt) (`self.findBT` points))
  (if _doesexist
    (`/Game/Lane/BridgeTunnel/BP_BridgeTunnel.countUp` (`.BridgeTunnelREF_6_8B3FBE7C45F28147E6CD329AFF428C26` (break `/Game/Lane/BridgeTunnel/ST_BT` _thebnt)))
    (else
      (`self.CreateNewBT` points))))

(event `self.DisconnectBT`
  (params (points :type "Array of IntPoint Structure (by ref)"))
  (`parent.DisconnectBT` points)
  (bind (_doesexist _thebnt) (`self.findBT` points))
  (if _doesexist
    (`/Game/Lane/BridgeTunnel/BP_BridgeTunnel.countDown` (`.BridgeTunnelREF_6_8B3FBE7C45F28147E6CD329AFF428C26` (break `/Game/Lane/BridgeTunnel/ST_BT` _thebnt)))
    (else
      (`KismetSystemLibrary.PrintString` "That disconnecting BNT doesnt Exist"))))

(fn `findBT`
  (params (findPoint :type "Array of IntPoint Structure"))
  (returns (doesExist :type Boolean) (theBNT :type "/Game/Lane/BridgeTunnel/ST_BT Structure"))
  (locals (reverse :type "Array of IntPoint Structure"))
  (bind _output_get (set `local.reverse` findPoint))
  (`KismetArrayLibrary.Array_Reverse` _output_get)
  (for _array_element (`self.BNT`)
    (if (or (`KismetArrayLibrary.Array_Identical` findPoint (break `ConnectorData` _array_element)) (`KismetArrayLibrary.Array_Identical` (`local.reverse`) (break `ConnectorData` _array_element)))
      (return true (make `/Game/Lane/BridgeTunnel/ST_BT` (break `ConnectorData` _array_element) "NewEnumerator0" null))))
  (return false))

(fn `UserConstructionScript`)