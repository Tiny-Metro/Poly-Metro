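; Bridge or tunnel connector actor that SetBNT builds along grid points and registers with its BTManager.
; Grid points become world locations on a linear spline, tiled with type-specific spline meshes and capped by outward-facing entrance meshes.
; A use count destroys the actor at zero after notifying the manager.
; CreatePointArray, not called here, derives a path with at most one bend between two entrances.
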(event `SetBNT`
  (params (GridREF :type "GridManager Object Reference") (PointSet :type "Array of IntPoint Structure") (BTManager :type "/Game/Lane/BridgeTunnel/BP_BridgeTunnelManger Object Reference") (ConnectorType :type "ConnectorType Enum" :default "Bridge"))
  ;[1 1 1] SetBNT
  (set `self.ConnectorData` (make `ConnectorData` PointSet ConnectorType self))
  (set `self.BTManagerREF` BTManager)
  (set `self.GridManagerRef` GridREF)
  (set `self.count` 1)
  (`self.BuildBridgeTunnel`))

(event `BuildBridgeTunnel`
  (bind (_connectordata_pointarr _connectordata_type) (break `ConnectorData` (`self.ConnectorData`)))
  (bind _connectordata_pointarr_2 (break `ConnectorData` (`self.ConnectorData`)))
  ;[1 1 1] BUILD
  (`self.setTunnelBridge` _connectordata_type)
  (bind _vecarray (`self.CreateLocArray` _connectordata_pointarr_2))
  (`self.MakeSpline` _vecarray)
  (`self.SetStrat/End` _vecarray)
  (`self.Register`))

(event `Register`
  (`/Game/Lane/BridgeTunnel/BP_BridgeTunnelManger.getRegister` (`self.BTManagerREF`) (`self.ConnectorData`)))

(event `countDown`
  (bind _output_get (set `self.count` (- (`self.count`) 1)))
  (if (< _output_get 1)
    (`self.SendDeathCertificate`)
    (`self.K2_DestroyActor`)))

(event `countUp`
  (set `self.count` (+ (`self.count`) 1)))

(event `destory`
  (`self.K2_DestroyActor`))

(event `SendDeathCertificate`
  (`/Game/Lane/BridgeTunnel/BP_BridgeTunnelManger.getDeathCertificate` (`self.BTManagerREF`) (`self.ConnectorData`)))

(fn `CreateLocArray`
  (params (PointArray :type "Array of IntPoint Structure"))
  (returns (VecArray :type "Array of Vector Structure"))
  (locals (VectorArray :type "Array of Vector Structure"))
  (bind _vectorarray (`local.VectorArray`))
  (for _array_element PointArray
    (bind (_returnvalue_index _returnvalue_worldcoordination _returnvalue_worldlocation) (break `GridCellData` (`GridManager.GetGridCellDataByPoint` (`self.GridManagerRef`) (break `IntPoint` _array_element) (`.Y` (break `IntPoint` _array_element)))))
    (`KismetArrayLibrary.Array_Add` _vectorarray _returnvalue_worldlocation))
  (return _vectorarray))

(fn `CreatePointArray`
  (params (Enterance0 :type "IntPoint Structure") (Enterance1 :type "IntPoint Structure"))
  (returns (PointArray :type "Array of IntPoint Structure"))
  (locals (intPointArray :type "Array of IntPoint Structure") (Enterance0Point :type "IntPoint Structure") (Enterance1Point :type "IntPoint Structure") (BendPoint :type "IntPoint Structure") (tmpPointArray :type "Array of IntPoint Structure"))
  (bind (_enterance0point_x _enterance0point_y) (break `IntPoint` (`local.Enterance0Point`)))
  (bind (_enterance1point_x _enterance1point_y) (break `IntPoint` (`local.Enterance1Point`)))
  (set `local.Enterance0Point` Enterance0)
  (set `local.Enterance1Point` Enterance1)
  (bind (_x _y _no_bend) (`self.FindBendInt` _enterance0point_x _enterance0point_y _enterance1point_x _enterance1point_y))
  (if _no_bend
    (`KismetArrayLibrary.Array_Add` (`local.tmpPointArray`) (`local.Enterance0Point`))
    (`KismetArrayLibrary.Array_Add` (`local.tmpPointArray`) (`local.Enterance1Point`))
    (else
      (set `local.BendPoint` (make `IntPoint` _x _y))
      (`KismetArrayLibrary.Array_Add` (`local.tmpPointArray`) (`local.Enterance0Point`))
      (`KismetArrayLibrary.Array_Add` (`local.tmpPointArray`) (`local.BendPoint`))
      (`KismetArrayLibrary.Array_Add` (`local.tmpPointArray`) (`local.Enterance1Point`))))
  (return (`local.tmpPointArray`)))

(fn `FindBendInt`
  (params (Xstart :type Integer) (Ystart :type Integer) (Xend :type Integer) (Yend :type Integer))
  (returns (X :type Integer) (Y :type Integer) (`no Bend` :type Boolean))
  (locals (Xdistance :type Integer) (Ydistance :type Integer))
  (bind _ydistance (`local.Ydistance`))
  (bind _xdistance (`local.Xdistance`))
  ;[1 1 1] if X = or Y=, then no Bend
  (if (== Ystart Yend)
    _
    (elif (== Xstart Xend)
      _
      (else
        ;[1 1 1] Set X, Ydistance
        (bind _output_get (set `local.Xdistance` (- Xend Xstart)))
        (bind _output_get_2 (set `local.Ydistance` (- Yend Ystart)))
        ;[1 1 1] if |Xd| == |Yd|, then no Bend
        (if (== (`KismetMathLibrary.Abs_Int` _output_get) (`KismetMathLibrary.Abs_Int` _output_get_2))
          (return 0 0 true)
          (else
            ;[1 0.8228 0.1144] |Xd| > |Yd|
            (if (> (`KismetMathLibrary.Abs_Int` (`local.Xdistance`)) (`KismetMathLibrary.Abs_Int` (`local.Ydistance`)))
              ;;[1 1 1] Same + / - ?
              (if (> (* (`local.Xdistance`) (`local.Ydistance`)) 0)
                ;;;[1 1 1] same +/-
                (return (- Xend (- (`local.Xdistance`) (`local.Ydistance`))) Yend false)
                (else
                  ;;;[1 1 1] different
                  (return (- Xstart _ydistance) (+ _ydistance Ystart) false)))
              (else
                ;[1 0.8228 0.1144] |Xd| < |Yd|
                ;;[1 1 1] Same + / - ?
                (if (> (* (`local.Xdistance`) (`local.Ydistance`)) 0)
                  ;;;[1 1 1] same +/-
                  (return Xend (- Yend (- (`local.Ydistance`) (`local.Xdistance`))) false)
                  (else
                    ;;;[1 1 1] different
                    (return (- Xstart _xdistance) (+ _xdistance Ystart) false))))))))))
  (return 0 0 true))

(fn `Get End Pos/Tangent`
  (params (Index :type Integer))
  (returns (Position :type "Vector Structure") (Tangent :type "Vector Structure"))
  (bind _spline (`self.Spline`))
  (bind _sectionlength (`self.SectionLength`))
  (bind _returnvalue (* (+ Index 1) _sectionlength))
  (return (`SplineComponent.GetLocationAtDistanceAlongSpline` _spline _returnvalue "Local") (`KismetMathLibrary.ClampVectorSize` (`SplineComponent.GetTangentAtDistanceAlongSpline` _spline _returnvalue "Local") 0.0 _sectionlength)))

(fn `Get Start Pos/Tangent`
  (params (Index :type Integer))
  (returns (Position :type "Vector Structure") (Tangent :type "Vector Structure"))
  (bind _sectionlength (`self.SectionLength`))
  (bind _spline (`self.Spline`))
  (bind _returnvalue (* Index _sectionlength))
  (return (`SplineComponent.GetLocationAtDistanceAlongSpline` _spline _returnvalue "Local") (`KismetMathLibrary.ClampVectorSize` (`SplineComponent.GetTangentAtDistanceAlongSpline` _spline _returnvalue "Local") 0.0 _sectionlength)))

(fn `MakeSpline`
  (params (VecArray :type "Array of Vector Structure"))
  (locals (VectorArray :type "Array of Vector Structure"))
  (`SplineComponent.SetSplinePoints` (`self.Spline`) VecArray "World" true)
  (for (_ _array_index) VecArray
    (`SplineComponent.SetSplinePointType` (`self.Spline`) _array_index "Linear" true))
  (for _index (range (`KismetMathLibrary.FTrunc` (/ (`SplineComponent.GetSplineLength` (`self.Spline`)) (`self.SectionLength`))))
    (bind _returnvalue (`AddComponent|NODE_AddSplineMeshComponent-0`))
    (`StaticMeshComponent.SetStaticMesh` _returnvalue (`self.MiddleMesh`))
    (`SplineMeshComponent.SetForwardAxis` _returnvalue "X" true)
    (bind (_position _tangent) (`self.Get Start Pos/Tangent` _index))
    (bind (_position_2 _tangent_2) (`self.Get End Pos/Tangent` _index))
    (`SplineMeshComponent.SetStartAndEnd` _returnvalue _position _tangent _position_2 _tangent_2 true))
  (return))

(fn `SetStrat/End`
  (params (vectorPoints :type "Array of Vector Structure"))
  (bind _returnvalue (`KismetArrayLibrary.Array_LastIndex` vectorPoints))
  (bind _output (`|GetArrayItem` vectorPoints))
  (bind _enterance1mesh (`self.Enterance1Mesh`))
  (bind _enterance0mesh (`self.Enterance0Mesh`))
  (bind _output_2 (`|GetArrayItem` vectorPoints _returnvalue))
  (`PrimitiveComponent.SetCollisionEnabled` _enterance1mesh "NoCollision")
  (`SceneComponent.K2_SetWorldLocationAndRotation` _enterance1mesh _output_2 (`KismetMathLibrary.Conv_VectorToRotator` (- _output_2 (`|GetArrayItem` vectorPoints (- _returnvalue 1)))) false false)
  (`PrimitiveComponent.SetCollisionEnabled` _enterance0mesh "NoCollision")
  (`SceneComponent.K2_SetWorldLocationAndRotation` _enterance0mesh _output (`KismetMathLibrary.Conv_VectorToRotator` (- _output (`|GetArrayItem` vectorPoints 1))) false false)
  (return))

(fn `setTunnelBridge`
  (params (ConnectorType :type "ConnectorType Enum" :default "Bridge"))
  (switch `ConnectorType` ConnectorType
    (:`Bridge`
      (set `self.SectionLength` 76.0)
      (`StaticMeshComponent.SetStaticMesh` (`self.Enterance1Mesh`) "/Game/Lane/BridgeTunnel/SM_BridgeParted.SM_BridgeParted")
      (`StaticMeshComponent.SetStaticMesh` (`self.Enterance0Mesh`) "/Game/Lane/BridgeTunnel/SM_BridgeParted.SM_BridgeParted")
      (set `self.MiddleMesh` "/Game/Lane/BridgeTunnel/SM_BridgeParted.SM_BridgeParted"))
    (:`Tunnel`
      (set `self.SectionLength` 87.0)
      (`StaticMeshComponent.SetStaticMesh` (`self.Enterance1Mesh`) "/Game/Lane/BridgeTunnel/SM_TunnelEnterance.SM_TunnelEnterance")
      (`StaticMeshComponent.SetStaticMesh` (`self.Enterance0Mesh`) "/Game/Lane/BridgeTunnel/SM_TunnelEnterance.SM_TunnelEnterance")
      (set `self.MiddleMesh` "/Game/Lane/BridgeTunnel/SM_TunnelMiddle.SM_TunnelMiddle")))
  (return))

(fn `UserConstructionScript`)