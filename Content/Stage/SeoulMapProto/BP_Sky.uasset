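; Sky actor that runs a looping day-night cycle with a cube sky mesh and a directional light.
; Construction creates a dynamic M_Sky instance and passes it Time, Step and the day length.
; Tick accumulates Time, feeds it to the material, and updates the light.
; Time modulo DaySecond selects one of four equal phases, each lerping sun rotation and color, with intensity halved in the last two.
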(event `self.ReceiveTick`
  (params (DeltaSeconds :type "Float (single-precision)"))
  (bind _output_get (set `self.Time` (+ DeltaSeconds (`self.Time`))))
  (`MaterialInstanceDynamic.SetScalarParameterValue` (`self.SkyMaterial`) "Time" _output_get)
  (`self.SetLightRotation`)
  (`SceneComponent.K2_SetWorldRotation` (`self.DirectionalLight`) (`self.LightRotation`) false false)
  (`LightComponent.SetLightColor` (`self.DirectionalLight`) (`self.SunLightColor`) true))

(event `SetLightRotation`
  (bind _daysecond (`self.DaySecond`))
  (bind _returnvalue (* (/ (`KismetMathLibrary.FMod` (`self.Time`) _daysecond) _daysecond) 4.0))
  (bind _returnvalue_2 (- _returnvalue 1.0))
  (bind _returnvalue_3 (- _returnvalue_2 1.0))
  (bind _returnvalue_4 (- _returnvalue_3 1.0))
  (if (< _returnvalue 1.0)
    (set `self.LightRotation` (`KismetMathLibrary.RLerp` (struct :`Yaw` 180.0) (struct :`Pitch` -70.0 :`Yaw` 270.0) _returnvalue))
    (set `self.SunLightColor` (`KismetMathLibrary.LinearColorLerp` (struct :`R` 1.0 :`G` 0.262251 :`A` 1.0) (struct :`R` 0.654832 :`G` 0.970118 :`B` 1.0 :`A` 1.0) _returnvalue))
    (`LightComponent.SetIntensity` (`self.DirectionalLight`) 1.0 :!label _label)
    (elif (< _returnvalue_2 1.0)
      (set `self.LightRotation` (`KismetMathLibrary.RLerp` (struct :`Pitch` -70.0 :`Yaw` 270.0) (struct :`Yaw` 360.0) _returnvalue_2))
      (set `self.SunLightColor` (`KismetMathLibrary.LinearColorLerp` (struct :`R` 0.651406 :`G` 0.973445 :`B` 1.0 :`A` 1.0) (struct :`R` 1.0 :`G` 0.046665 :`B` 0.313989 :`A` 1.0) _returnvalue_2))
      (goto _label)
      (elif (< _returnvalue_3 1.0)
        (set `self.LightRotation` (`KismetMathLibrary.RLerp` (struct) (struct :`Pitch` -20.0 :`Yaw` 90.0) _returnvalue_3))
        (set `self.SunLightColor` (`KismetMathLibrary.LinearColorLerp` (struct :`R` 1.0 :`G` 0.046665 :`B` 0.313989 :`A` 1.0) (struct :`G` 0.068574 :`B` 1.0 :`A` 1.0) _returnvalue_3))
        (`LightComponent.SetIntensity` (`self.DirectionalLight`) 0.5 :!label _label_2)
        (elif (< _returnvalue_4 1.0)
          (set `self.LightRotation` (`KismetMathLibrary.RLerp` (struct :`Pitch` -20.0 :`Yaw` 90.0) (struct :`Yaw` 180.0) _returnvalue_4))
          (set `self.SunLightColor` (`KismetMathLibrary.LinearColorLerp` (struct :`G` 0.068478 :`B` 1.0 :`A` 1.0) (struct :`R` 1.0 :`G` 0.262251 :`A` 1.0) _returnvalue_4))
          (goto _label_2))))))

(fn `UserConstructionScript`
  (bind _returnvalue (`PrimitiveComponent.CreateDynamicMaterialInstance` (`self.M_CubeSky`) 0 "/Game/Stage/SeoulMapProto/M_Sky.M_Sky" "Time"))
  (bind _output_get (set `self.SkyMaterial` _returnvalue))
  (`MaterialInstanceDynamic.SetScalarParameterValue` _returnvalue "Time" (`self.Time`))
  (`MaterialInstanceDynamic.SetScalarParameterValue` _output_get "Time" (`self.Time`))
  (`MaterialInstanceDynamic.SetScalarParameterValue` _returnvalue "Step" (`KismetMathLibrary.Conv_IntToDouble` (`self.Step`)))
  (`MaterialInstanceDynamic.SetScalarParameterValue` _returnvalue "DivideTime" (`self.DaySecond`)))