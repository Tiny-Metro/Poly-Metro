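; Stage HUD controller that creates the player HUD and game-over widgets and tracks play time, money and the current event.
; Tick advances time unless the clock widget is paused, doubling it on fast-forward and printing debug values.
; Number keys act as test inputs that switch event text or adjust money.
; Money below a negative limit, or the C key, ends the game, replacing all widgets with the game-over window.
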(event `SetGameOver`
  (params (gameOverFlag :type Integer))
  (bind _gameoverwindowreference (`self.GameOverWindowReference`))
  (set `self.IsGameOver` true)
  (`KismetSystemLibrary.PrintString` "GAMEOVER")
  (`/Game/Stage/UI/HUD/WBP_GameOverWindow.SetGameOverConditionTxt` _gameoverwindowreference gameOverFlag)
  (`WidgetLayoutLibrary.RemoveAllWidgets`)
  (`UserWidget.AddToViewport` _gameoverwindowreference 0))

(event `self.ReceiveBeginPlay`
  ;[1 0.8812 0.3277] Initializing
  (set `self.IsGameOver` false)
  (bind _returnvalue (`|CreateWidget` "/Game/Stage/UI/HUD/WBP_UserHUD.WBP_UserHUD_C"))
  (`UserWidget.AddToViewport` _returnvalue 0)
  (bind _output_get (set `self.MoneyReference` _returnvalue))
  (`/Game/Stage/UI/HUD/WBP_EventWindow.updateEventTxt` (`/Game/Stage/UI/HUD/WBP_UserHUD.EventWindowReference` _output_get) (`self.StrEvent`))
  (bind _returnvalue_2 (`|CreateWidget` "/Game/Stage/UI/HUD/WBP_GameOverWindow.WBP_GameOverWindow_C"))
  (set `self.GameOverWindowReference` _returnvalue_2))

(event `PlayTime`
  ;[1 1 1] Time
  (if (`/Game/Stage/UI/HUD/WBP_ClockToggle.isFastForward` (`/Game/Stage/UI/HUD/WBP_UserHUD.ClockWidgetReference` (`self.MoneyReference`)))
    (set `self.Time` (+ (`self.Time`) (* 2.0 (`self.DeltaTime`))))
    (`KismetSystemLibrary.PrintString` (`KismetStringLibrary.Conv_DoubleToString` (`self.Time`)))
    (`KismetSystemLibrary.PrintString` (`KismetStringLibrary.Conv_DoubleToString` (`self.DeltaTime`)) true true (struct :`R` 1.0 :`G` 0.304653 :`B` 0.404501 :`A` 1.0))
    (else
      (set `self.Time` (+ (`self.Time`) (`self.DeltaTime`)))
      (`KismetSystemLibrary.PrintString` (`KismetStringLibrary.Conv_DoubleToString` (`self.Time`)))
      (`KismetSystemLibrary.PrintString` (`KismetStringLibrary.Conv_DoubleToString` (`self.DeltaTime`)) true true (struct :`R` 1.0 :`G` 0.246464 :`B` 0.316203 :`A` 1.0)))))

(event `Key|One`
  (params (Key :type "Key Structure"))
  ;[1 0.5207 0.8591] currentEvent
  (:`Pressed`
    (`/Game/Stage/UI/HUD/WBP_UserHUD.updateCurrentEvent` (`self.MoneyReference`) (`|GetArrayItem` (`self.TxtEvent`)))))

(event `Key|Two`
  (params (Key :type "Key Structure"))
  ;[1 0.5207 0.8591] currentEvent
  (:`Pressed`
    (`/Game/Stage/UI/HUD/WBP_UserHUD.updateCurrentEvent` (`self.MoneyReference`) (`|GetArrayItem` (`self.TxtEvent`) 1))))

(event `Key|Three`
  (params (Key :type "Key Structure"))
  ;[1 0.5207 0.8591] currentEvent
  (:`Pressed`
    (`/Game/Stage/UI/HUD/WBP_UserHUD.updateCurrentEvent` (`self.MoneyReference`) (`|GetArrayItem` (`self.TxtEvent`) 2))))

(event `Key|Four`
  (params (Key :type "Key Structure"))
  ;[1 0.5207 0.8591] currentEvent
  (:`Pressed`
    (`/Game/Stage/UI/HUD/WBP_UserHUD.updateCurrentEvent` (`self.MoneyReference`) (`|GetArrayItem` (`self.TxtEvent`) 3))))

(event `self.ReceiveTick`
  (params (DeltaSeconds :type "Float (single-precision)"))
  ;[1 1 1] Time
  (if (not (`self.IsGameOver`))
    (set `self.DeltaTime` DeltaSeconds)
    (if (`/Game/Stage/UI/HUD/WBP_ClockToggle.IsPasued` (`/Game/Stage/UI/HUD/WBP_UserHUD.ClockWidgetReference` (`self.MoneyReference`)))
      (`self.timeStop`)
      (else
        (`self.PlayTime`)))))

(event `timeStop`
  ;[1 1 1] Time
  (`KismetSystemLibrary.PrintString` (`KismetStringLibrary.Conv_DoubleToString` (`self.Time`)))
  ;[1 0.5207 0.8591] currentEvent
  (`KismetSystemLibrary.PrintString` (`KismetStringLibrary.Conv_DoubleToString` (`self.DeltaTime`)) true true (struct :`R` 1.0 :`G` 0.246464 :`B` 0.316203 :`A` 1.0)))

(event `Key|Zero`
  (params (Key :type "Key Structure"))
  ;[0.4409 1 0.2645] Money
  (:`Pressed`
    (if (not (`self.IsGameOver`))
      (set `self.Money` (+ (`self.Money`) 10.0))
      (`/Game/Stage/UI/HUD/WBP_UserHUD.updateMoney` (`self.MoneyReference`) (`self.Money`) :!label _label)
      (if (< (`self.Money`) -10.0)
        (`self.setGameOver` 1)))))

(event `Key|C`
  (params (Key :type "Key Structure"))
  ;[1 0.1146 0.1146] complain
  (:`Pressed`
    (`self.setGameOver` 0)))

(event `Key|Nine`
  (params (Key :type "Key Structure"))
  ;[0.4409 1 0.2645] Money
  (:`Pressed`
    (if (not (`self.IsGameOver`))
      (set `self.Money` (- (`self.Money`) 10.0))
      (goto _label))))

(fn `UserConstructionScript`)