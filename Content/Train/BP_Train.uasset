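; BP_Train is an AI-controlled train that begins patrolling when its ServiceStart event supplies a start location.
; BeginPlay caches its BP_TrainAiController, and ServiceStart passes the location to SetTestRoutine before calling Patrol on it.
; Overlap with a BP_Lane and touch input only print debug text.
; Clicking looks up the BP_RtsCamera but does nothing with it yet.
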(event `ServiceStart`
  (params (StartLocation :type "Vector Structure"))
  (bind _aicontrollerref (`self.AiControllerRef`))
  (`/Game/Train/BP_TrainAiController.SetTestRoutine` _aicontrollerref StartLocation)
  (`/Game/Train/BP_TrainAiController.Patrol` _aicontrollerref)
  (`KismetSystemLibrary.PrintText` "Service Start"))

(event `self.ReceiveBeginPlay`
  (bind _asbp_train_ai_controller (cast `/Game/Train/BP_TrainAiController` (`AIBlueprintHelperLibrary.GetAIController` self))
    (:`then`
      (set `self.AiControllerRef` _asbp_train_ai_controller))
    (:`CastFailed`
      (`KismetSystemLibrary.PrintText` "Cast Fail : Train Ai Controller"))))

(event `self.ReceiveActorBeginOverlap`
  (params (OtherActor :type "Actor Object Reference"))
  (bind _asbp_lane (cast `/Game/TrackLine/BP_Lane` OtherActor)
    (:`then`
      (`KismetSystemLibrary.PrintString` "Hello")
      (`KismetSystemLibrary.PrintString` (`KismetSystemLibrary.GetDisplayName` _asbp_lane) true true (struct :`R` 1.0 :`B` 0.057804 :`A` 1.0)))
    (:`CastFailed`
      (`KismetSystemLibrary.PrintString` "castFailed"))))

(event `self.ReceiveActorEndOverlap`
  (params (OtherActor :type "Actor Object Reference")))

(event `self.ReceiveActorOnInputTouchBegin`
  (params (FingerIndex :type "ETouchIndex Enum" :default "Touch1"))
  (`KismetSystemLibrary.PrintString` "Touch"))

(event `self.ReceiveActorOnClicked`
  (params (ButtonPressed :type "Key Structure"))
  (`GameplayStatics.GetActorOfClass` "/Game/Camera/BP_RtsCamera.BP_RtsCamera_C"))

(fn `UserConstructionScript`)