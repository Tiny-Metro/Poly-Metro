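; AI controller for a subtrain that follows a target train at a set distance.
; Its Follow event measures the navigation path length from the controlled pawn to TargetTrain.
; Unless that length is under DistanceFromTrain, it prints debug text and moves to the train, using the same distance as acceptance radius.
; Nothing in this graph calls Follow, and an AIMoveTo node is left unconnected.
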(event `self.ReceiveBeginPlay`)

(event `self.Follow`
  (bind _distancefromtrain (`self.DistanceFromTrain`))
  (if (not (< (`NavigationSystemV1.GetPathLength` (`self.K2_GetActorLocation` (`self.K2_GetPawn`)) (`self.K2_GetActorLocation` (`self.TargetTrain`)) null "/Script/AIModule.NavFilter_AIControllerDefault") _distancefromtrain))
    (`KismetSystemLibrary.PrintText` "Hello")
    (`self.MoveToActor` (`self.TargetTrain`) _distancefromtrain true true true "/Script/AIModule.NavFilter_AIControllerDefault")))

(fn `UserConstructionScript`)