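; AI controller for BP_Train that caches the possessed train and stores the first BP_Station found as a test target.
; Patrol, not started by any live event here, runs AIMoveTo toward TrainDestination unless the train is dragged, re-calling itself on success or failure.
; SetTestRoutine builds a list of offset test waypoints that Patrol does not read.
; The next-destination update and move-to-station test are disconnected.
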(event `self.ReceivePossess`
  (params (PossessedPawn :type "Pawn Object Reference"))
  (`KismetSystemLibrary.PrintString` "Possess")
  (bind _asbp_train (cast `/Game/Train/BP_Train` (`self.K2_GetPawn`)))
  (set `self.TrainRef` _asbp_train)
  (bind _outactors (`GameplayStatics.GetAllActorsOfClass` "/Game/Station/BP_Station.BP_Station_C"))
  (set `self.TestTarget` (`|GetArrayItem` _outactors)))

(event `self.ReceiveTick`
  (params (DeltaSeconds :type "Float (single-precision)")))

(event `self.Patrol`
  (if (not (`TrainTemplate.IsActorDragged` (`self.TrainRef`)))
    (`KismetSystemLibrary.PrintString` "TrainController:Patrol")
    (bind _movementresult (`|AIMoveTo` (`Pawn.GetController` (`self.K2_GetPawn`)) null (`self.TrainDestination`) null 100.0)
      (:`OnSuccess`
        _)
      (:`OnFail`
        _))
    (`self.Patrol`)))

(event `SetTestRoutine`
  (params (StartLocation :type "Vector Structure"))
  (`KismetArrayLibrary.Array_Add` (`self.TestRoutine`) StartLocation)
  (for _index (range 4)
    (`KismetArrayLibrary.Array_Add` (`self.TestRoutine`) (+ StartLocation (`KismetMathLibrary.MakeVector` (`KismetMathLibrary.Conv_IntToDouble` (* _index 400))))))
  (for _index_2 (range 4)
    (`KismetArrayLibrary.Array_Add` (`self.TestRoutine`) (+ (`|GetArrayItem` (`self.TestRoutine`) _index_2) (`KismetMathLibrary.MakeVector` 0.0 (`KismetMathLibrary.Conv_IntToDouble` (* _index_2 400)))))))

(fn `UserConstructionScript`)