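; BP_TinyMetroCamera is a spring-arm camera pawn sketched for player-driven move, zoom and rotation, but none of its logic runs.
; BeginPlay and Tick are empty, and every input-handling fragment is disconnected from an event.
; Those fragments outline Enhanced Input mapping, drag panning via DefineMoveDirection, arm-length zoom, and click timing for long-click rotation mode and double-click.
; Rotation uses placeholder values, and DoubleClick only prints a debug string.
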(event `self.ReceiveBeginPlay`)

(event `self.ReceiveTick`
  (params (DeltaSeconds :type "Float (single-precision)")))

(event `EnhancedInput|/Game/Camera/Input/IA_CameraZoom`
  (params (ActionValue :type "Float (double-precision)") (ElapsedSeconds :type "Float (double-precision)") (TriggeredSeconds :type "Float (double-precision)") (InputAction :type "InputAction Object Reference" :default "/Game/Camera/Input/IA_CameraZoom.IA_CameraZoom")))

(event `EnhancedInput|/Game/Camera/Input/IA_CameraRotation`
  (params (ActionValue :type "Float (double-precision)") (ElapsedSeconds :type "Float (double-precision)") (TriggeredSeconds :type "Float (double-precision)") (InputAction :type "InputAction Object Reference" :default "/Game/Camera/Input/IA_CameraRotation.IA_CameraRotation")))

(event `EnhancedInput|/Game/Camera/Input/IA_CameraMove`
  (params (ActionValue :type "Vector2D Structure") (ElapsedSeconds :type "Float (double-precision)") (TriggeredSeconds :type "Float (double-precision)") (InputAction :type "InputAction Object Reference" :default "/Game/Camera/Input/IA_CameraMove.IA_CameraMove")))

(event `EnhancedInput|/Game/Camera/Input/IA_ToggleCameraRotation`
  (params (ActionValue :type Boolean) (ElapsedSeconds :type "Float (double-precision)") (TriggeredSeconds :type "Float (double-precision)") (InputAction :type "InputAction Object Reference" :default "/Game/Camera/Input/IA_ToggleCameraRotation.IA_ToggleCameraRotation"))
  ;[1 1 1] Long Click : Toggle camera rotation mode
)

(event `EnhancedInput|/Game/Camera/Input/IA_CameraMove`
  (params (ActionValue :type "Vector2D Structure") (ElapsedSeconds :type "Float (double-precision)") (TriggeredSeconds :type "Float (double-precision)") (InputAction :type "InputAction Object Reference" :default "/Game/Camera/Input/IA_CameraMove.IA_CameraMove")))

(event `EnhancedInput|/Game/Camera/Input/IA_DoubleTab`
  (params (ActionValue :type Boolean) (ElapsedSeconds :type "Float (double-precision)") (TriggeredSeconds :type "Float (double-precision)") (InputAction :type "InputAction Object Reference" :default "/Game/Camera/Input/IA_DoubleTab.IA_DoubleTab"))
  ;[1 1 1] Double Click : Cam rotation init
)

(fn `DefineMoveDirection`
  (params (Start :type "Vector2D Structure") (Current :type "Vector2D Structure"))
  (returns (NewParam :type "Vector Structure"))
  (bind (_returnvalue_x _returnvalue_y) (`KismetMathLibrary.BreakVector2D` (`KismetMathLibrary.Normal2D` (- Start Current))))
  (return (`KismetMathLibrary.MakeVector` _returnvalue_x _returnvalue_y)))

(fn `DoubleClick`
  (`KismetSystemLibrary.PrintString` "DoubleClick!"))

(fn `UserConstructionScript`)