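; BP_RtsCamera is an RTS camera Blueprint holding an unfinished camera reset feature, with no logic that runs.
; Unconnected ResetCameraPosition fragments sketch a timeline that lerps control rotation to the Arrow component's rotation along the shortest path.
; Other orphaned nodes set a CameraResetting flag and use it to gate a yaw input that is multiplied by zero.
; BeginPlay, overlap and the construction script are empty.
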(event `InputAction|ResetCamera`
  (params (Key :type "Key Structure"))
  ;[1 1 1] ResetCameraPosition
)

(fn `UserConstructionScript`)