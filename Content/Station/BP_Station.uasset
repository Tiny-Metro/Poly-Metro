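; BP_Station is a station actor that shows its state through three text displays.
; Every Tick it writes the station type enum's name, the current complaint value and the number of entries in its Passenger array to those texts.
; The graph only refreshes the display; BeginPlay, overlap and the construction script are empty, and nothing here changes the underlying values.
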(event `self.ReceiveTick`
  (params (DeltaSeconds :type "Float (single-precision)"))
  (`TextRenderComponent.K2_SetText` (`self.Type`) (`KismetTextLibrary.Conv_StringToText` (`|GetEnumeratorNameAsString` (`self.StationTypeValue`))))
  (`TextRenderComponent.K2_SetText` (`self.Complain`) (`KismetTextLibrary.Conv_IntToText` (`self.ComplainCurrent`)))
  (`TextRenderComponent.K2_SetText` (`self.NumOfPassenger`) (`KismetTextLibrary.Conv_IntToText` (`KismetArrayLibrary.Array_Length` (`self.Passenger`)))))

(fn `UserConstructionScript`)