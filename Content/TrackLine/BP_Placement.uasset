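; BP_Placement is a placement preview actor that follows the mouse cursor in the world.
; Each Tick it applies MeshType to its StaticMesh, line-traces from the deprojected cursor, and moves to the hit's XY at a fixed height.
; A right-click destroys it.
; UpdateCollision, which applies a "not possible" material when nothing overlaps, is never called.
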(event `self.ReceiveActorBeginOverlap`
  (params (OtherActor :type "Actor Object Reference")))

(event `self.ReceiveTick`
  (params (DeltaSeconds :type "Float (single-precision)"))
  (bind (_worldlocation _worlddirection) (`PlayerController.DeprojectMousePositionToWorld` (`GameplayStatics.GetPlayerController` 0)))
  (`StaticMeshComponent.SetStaticMesh` (`self.StaticMesh`) (`self.MeshType`))
  (bind _outhit (`KismetSystemLibrary.LineTraceSingle` _worldlocation (+ _worldlocation (* _worlddirection (100000.0 100000.0 100000.0))) "TraceTypeQuery1"))
  (`self.K2_SetActorLocation` (`KismetMathLibrary.MakeVector` (.x (`.Location` (`GameplayStatics.BreakHitResult` _outhit))) (.y (`.Location` (`GameplayStatics.BreakHitResult` _outhit))) 20.0))
  (if (`PlayerController.WasInputKeyJustPressed` (`GameplayStatics.GetPlayerController` 0) "RightMouseButton")
    (`self.K2_DestroyActor`)))

(fn `UpdateCollision`
  (if (== (`KismetArrayLibrary.Array_Length` (`self.GetOverlappingActors` null)) 0)
    (`PrimitiveComponent.SetMaterial` (`self.StaticMesh`) 0 "/Game/TrackLine/M_NotPossible.M_NotPossible")
    (return)))

(fn `UserConstructionScript`)